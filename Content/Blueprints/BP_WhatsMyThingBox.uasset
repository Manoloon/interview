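; Trigger box checkpoint that sorts overlapping planet citizens by identity or color name, set by TriggerBoxFunctionalities, showing the answer tinted in their color.
; Citizens are queried and redirected through BPI_PlanetCitizen, with the spaceship and color-check destination found at BeginPlay.
; The identity box sends Sphericons to the spaceship and others to a random point in the color box.
; The color box sends Blue citizens aboard, counting others as left behind and routing them to world origin.
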(event `self.ReceiveBeginPlay`
  ;[0.01982 0 1 0] Getting Reference to the Spaceship
  (bind _outactors (`GameplayStatics.GetAllActorsOfClass` "/Game/Blueprints/BP_InterGalacticShip.BP_InterGalacticShip_C"))
  (set `self.Spaceship` (`|GetArrayItem` _outactors))
  ;[0.01982 0 1 0] Getting Reference of WhatsMyThingBox
  (bind _outactors_2 (`GameplayStatics.GetAllActorsOfClass` "BP_WhatsMyThingBox_C"))
  (for _array_element _outactors_2
    ;[1 0 0.2376 0] If is Color Check Point -> Set a random point inside his box -> this is used to send the citizens that are NOT Sphericons to check their color
    (if (`|EnumEquality` (`/Game/Blueprints/BP_WhatsMyThingBox.TriggerBoxFunctionalities` _array_element) "NewEnumerator0")
      (bind (_origin _boxextent) (`KismetSystemLibrary.GetComponentBounds` (`/Game/Blueprints/BP_WhatsMyThingBox.CollisionComp` _array_element)))
      (set `self.CheckingColorDestination` (`KismetMathLibrary.RandomPointInBoundingBox` _origin _boxextent)))))

(event `self.CollisionComp.OnComponentBeginOverlap`
  (params (OverlappedComponent :type "PrimitiveComponent Object Reference") (OtherActor :type "Actor Object Reference") (OtherComp :type "PrimitiveComponent Object Reference") (OtherBodyIndex :type Integer) (bFromSweep :type Boolean) (SweepResult :type "HitResult Structure (by ref)"))
  ;[0.01982 0 1 0] If Overlapping and implement interface : Get the color name , the identity and the linear Color and set the Actor Text
  (if (`KismetSystemLibrary.DoesImplementInterface` OtherActor "/Game/Interfaces/BPI_PlanetCitizen.BPI_PlanetCitizen_C")
    (`self.WhoIsOverlapping` OtherActor)))

(fn `UserConstructionScript`
  (bind _sometext (`self.SomeText`))
  (switch `/Game/Enums/E_TriggerBoxFunctionalities` (`self.TriggerBoxFunctionalities`)
    (:`NewEnumerator0`
      (`TextRenderComponent.K2_SetText` _sometext (`self.Text1`)))
    (:`NewEnumerator1`
      (`TextRenderComponent.K2_SetText` _sometext (`self.Text2`)))))

(fn `WhoIsOverlapping`
  (params (Actor :type "Actor Object Reference"))
  (bind _color (message `/Game/Interfaces/BPI_PlanetCitizen.BPI_WhatIsMyColor` Actor))
  (bind _colorname (message `/Game/Interfaces/BPI_PlanetCitizen.BPI_GetColorName` Actor))
  ;[0.01982 0 1 0] Are they Sphericons
  (bind _identity (message `/Game/Interfaces/BPI_PlanetCitizen.BPI_WhatIsMyIdentity` Actor))
  (if (`|EnumEquality` (`self.TriggerBoxFunctionalities`) "NewEnumerator1")
    (bind _returnvalue (`KismetMathLibrary.Conv_LinearColorToColor` _color))
    (`self.SetText` (`KismetTextLibrary.Conv_StringToText` _identity) _returnvalue)
    (if (`KismetStringLibrary.EqualEqual_StrStr` _identity "Sphericon")
      ;[1 0 0.2376 0] If they are Sphericons -> run toward the spaceship
      (bind _spaceship (`self.Spaceship` :!label _label)
        (:`then`
          (message `/Game/Interfaces/BPI_PlanetCitizen.BPI_SetDestination` Actor (`self.K2_GetActorLocation` _spaceship)))
        (:`else`))
      (else
        ;[1 0 0.2376 0] Send Citizen to check his Color
        (message `/Game/Interfaces/BPI_PlanetCitizen.BPI_SetDestination` Actor (`self.CheckingColorDestination`))))
    (else
      ;[0.01982 0 1 0] they are not sphericons , so are they blue¿?
      (`self.SetText` (`KismetTextLibrary.Conv_StringToText` _colorname) _returnvalue)
      (if (`KismetStringLibrary.EqualEqual_StrStr` _colorname "Blue")
        (goto _label)
        (else
          ;[1 0 0.2376 0] Count the citizen that are left behind
          (`/Game/Blueprints/BP_GameMode.SetLeftBehindCount` (`/Game/Blueprints/FunctionLibrary.GetGameModeBP`))
          (message `/Game/Interfaces/BPI_PlanetCitizen.BPI_SetDestination` Actor (0.0 0.0 0.0)))))))