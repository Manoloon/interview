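; BP_InterGalacticShip is an escape spaceship that boards qualifying citizens as survivors before taking off.
; A looping timer updates a countdown text that changes color in the final seconds.
; Capsule overlaps attach Sphericon or Blue BP_Citizens to the ship, disable their gravity and collision, and increment the GameMode survivor count.
; After the delay, it hides the text, disables boarding collision and rises via a timeline.
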(event `self.ReceiveBeginPlay`
  (bind (_returnvalue_x _returnvalue_y) (`KismetMathLibrary.BreakVector` (`self.K2_GetActorLocation`)))
  ;[0.01982 0 1 0] Set Timer
  (`KismetSystemLibrary.K2_SetTimer` null "SetCountText" 1.0 true)
  (`KismetSystemLibrary.Delay` 15.0)
  ;[0.01982 0 1 0] Spaceship take off
  (`SceneComponent.SetVisibility` (`self.TextRender`) false false)
  (`PrimitiveComponent.SetCollisionEnabled` (`self.Capsule`) "NoCollision")
  (bind (_direction _alpha) (`Timeline|Timeline_0` :!via `PlayFromStart`)
    (:`Update`
      (`self.K2_SetActorLocation` (`|EaseFunction` "Linear" _alpha (`self.K2_GetActorLocation`) (`KismetMathLibrary.MakeVector` _returnvalue_x _returnvalue_y 300.0))))))

(event `self.Capsule.OnComponentBeginOverlap`
  (params (OverlappedComponent :type "PrimitiveComponent Object Reference") (OtherActor :type "Actor Object Reference") (OtherComp :type "PrimitiveComponent Object Reference") (OtherBodyIndex :type Integer) (bFromSweep :type Boolean) (SweepResult :type "HitResult Structure (by ref)"))
  ;[0.01982 0 1 0] Counting Survivors / Only Sphericons or Blue ones! : They are attach to the hull of the spaceship
  (bind _asbp_citizen (cast `/Game/Blueprints/BP_Citizen` OtherActor))
  (bind _colorname (`/Game/Blueprints/BP_Citizen.BPI_GetColorName` _asbp_citizen))
  (bind _identity (`/Game/Blueprints/BP_Citizen.BPI_WhatIsMyIdentity` _asbp_citizen))
  (if (or (`KismetStringLibrary.EqualEqual_StrStr` _identity "Sphericon") (`KismetStringLibrary.EqualEqual_StrStr` _colorname "Blue"))
    (bind _capsulecomponent (`Character.CapsuleComponent` _asbp_citizen))
    (`PrimitiveComponent.SetEnableGravity` _capsulecomponent false)
    (`self.K2_AttachToActor` _asbp_citizen self "None" "SnapToTarget" "SnapToTarget" "SnapToTarget" false)
    (`PrimitiveComponent.SetCollisionEnabled` _capsulecomponent "NoCollision")
    ;[0 0.02507 1 0] Count it as Survivor
    (`/Game/Blueprints/BP_GameMode.SetSurvivorCount` (`/Game/Blueprints/FunctionLibrary.GetGameModeBP`))))

(fn `SetCountText`
  (bind _output_get (set `self.Count` (`KismetMathLibrary.Clamp` (- (`self.Count`) 1) 0 15)))
  (`TextRenderComponent.K2_SetText` (`self.TextRender`) (`KismetTextLibrary.Conv_IntToText` _output_get))
  (`TextRenderComponent.SetTextRenderColor` (`self.TextRender`) (`KismetMathLibrary.Conv_LinearColorToColor` (`KismetMathLibrary.SelectColor` (struct :`R` 0.630208 :`A` 1.0) (struct :`R` 1.0 :`G` 0.81279 :`B` 0.025944 :`A` 1.0) (<= (`self.Count`) 3)))))

(fn `UserConstructionScript`
  ;[0.01982 0 1 0] Set text with the Countdown
  (`TextRenderComponent.K2_SetText` (`self.TextRender`) (`KismetTextLibrary.Conv_IntToText` (`self.Count`))))