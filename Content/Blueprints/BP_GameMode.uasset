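; Game mode that tallies survivors and those left behind and runs the game-over sequence.
; Each Set count function increments its tally by one, and getters expose both totals.
; GameOver plays a brief slow motion via global time dilation and a delay, then restores normal speed, pauses the game and adds a WG_Stats widget to the viewport.
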(event `GameOver`
  (`GameplayStatics.SetGlobalTimeDilation` 0.25)
  (`KismetSystemLibrary.Delay` 0.5)
  (`GameplayStatics.SetGlobalTimeDilation` 1.0)
  (`GameplayStatics.SetGamePaused` true)
  (bind _returnvalue (`|CreateWidget` "/Game/Blueprints/WG_Stats.WG_Stats_C"))
  (bind _output_get (set `self.StatsUI` _returnvalue))
  (`UserWidget.AddToViewport` _output_get 0))

(fn `GetLeftBehind`
  (returns (LeftBehindCount :type Integer))
  (return (`self.LeftBehindCount`)))

(fn `GetSurvivors`
  (returns (SurvivorsCount :type Integer))
  (return (`self.SurvivorsCount`)))

(fn `SetLeftBehindCount`
  (set `self.LeftBehindCount` (+ (`self.LeftBehindCount`) 1)))

(fn `SetSurvivorCount`
  (set `self.SurvivorsCount` (+ (`self.SurvivorsCount`) 1)))

(fn `UserConstructionScript`)