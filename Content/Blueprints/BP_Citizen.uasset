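; BP_Citizen is an AI-moved citizen character with an identity and a color, which it carries to checks.
; An interface message sends it to a destination, flattened to Z=0, through SimpleMoveToLocation.
; Helper functions pull identity and shape from DT_Citizen, tint a dynamic material by color enum, label a text component with the color name, and randomize speed.
; Interface getters expose color name, color and identity.
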(event `/Game/Interfaces/BPI_PlanetCitizen.BPI_SetDestination`
  (params (Destination :type "Vector Structure"))
  ;[0 0.02507 1 0] Recieve the message of moving toward objective.
  (`self.MoveTowardCheck` (`KismetMathLibrary.MakeVector` Destination_X Destination_Y)))

(event `MoveTowardCheck`
  (params (Destination :type "Vector Structure"))
  ;[0.01982 0 1 0] Move Toward the check that he need to pass (identity and Color)
  (`AIBlueprintHelperLibrary.SimpleMoveToLocation` (`AIBlueprintHelperLibrary.GetAIController` self) (`KismetMathLibrary.MakeVector` Destination_X Destination_Y)))

(fn `BPI_GetColorName`
  (returns (ColorName :type String))
  (return (`self.ColorName`)))

(fn `BPI_WhatIsMyColor`
  (returns (Color :type "LinearColor Structure"))
  (return (`self.Color`)))

(fn `BPI_WhatIsMyIdentity`
  (returns (Identity :type String))
  (return (`self.Identity`)))

(fn `Getcolor`
  (returns (Color :type "LinearColor Structure"))
  (return (`self.Color`)))

(fn `GetColorName`
  (returns (ColorName :type String))
  (return (`self.ColorName`)))

(fn `SetBasicData`
  (returns (`Out Row Citizen Shape` :type "StaticMesh Object Reference"))
  ;[0.01982 0 1 0] Set Basic Data : Identity and Mesh for the Actor.
  (bind _returnvalue (`|GetDataTableRow` "/Game/Blueprints/DT_Citizen.DT_Citizen" (`KismetStringLibrary.Conv_StringToName` (`|GetEnumeratorNameAsString` (`self.CitizenType`))))
    (:`then`
      (`self.SetIdentity` (`|GetEnumeratorNameAsString` (break `/Game/Blueprints/ST_CitizenData` _returnvalue)))
      (return (`.citizenShape_7_43AEF4BF4C450E07AB85B4819665F59E` (break `/Game/Blueprints/ST_CitizenData` _returnvalue))))))

(fn `SetCitizenColor`
  (returns (Color :type "LinearColor Structure"))
  (switch `/Game/Enums/E_Colors` (`self.EColorName`)
    (:`NewEnumerator0`
      (set `self.Color` (struct)))
    (:`NewEnumerator1`
      (set `self.Color` (struct :`R` 0.01982 :`B` 1.0 :`A` 1.0)))
    (:`NewEnumerator2`
      (set `self.Color` (struct :`R` 0.062967 :`G` 1.0 :`A` 1.0)))
    (:`NewEnumerator3`
      (set `self.Color` (struct :`R` 1.0 :`A` 1.0)))
    (:`NewEnumerator4`
      (set `self.Color` (struct :`R` 1.0 :`G` 1.0 :`B` 1.0 :`A` 1.0))))
  (return (`self.Color`)))

(fn `SetColorName`
  (params (ColorName :type String))
  (set `self.ColorName` ColorName))

(fn `SetIdentity`
  (params (Identity :type String))
  (set `self.Identity` Identity))

(fn `SetMaterialDynamicSettings`
  (params (Target :type "PrimitiveComponent Object Reference"))
  (bind _returnvalue (`PrimitiveComponent.CreateDynamicMaterialInstance` Target 0 "/Game/Materials/M_CitizenColor.M_CitizenColor" "None"))
  (bind _color (`self.SetCitizenColor`))
  (`MaterialInstanceDynamic.SetVectorParameterValue` _returnvalue "Color" _color))

(fn `SetTextSettingsAndCharacterSpeed`
  (params (TextComp :type "TextRenderComponent Object Reference"))
  (bind _returnvalue (`KismetMathLibrary.RandomFloatInRange` 100.0 300.0))
  (bind _charactermovement (`self.CharacterMovement`))
  ;[0.01982 0 1 0] Set String of the color , and the Text of the actor
  (`self.SetColorName` (`|GetEnumeratorNameAsString` (`self.EColorName`)))
  (`TextRenderComponent.K2_SetText` TextComp (`KismetTextLibrary.Conv_StringToText` (`self.GetColorName`)))
  (`TextRenderComponent.SetTextRenderColor` TextComp (`KismetMathLibrary.Conv_LinearColorToColor` (`self.Getcolor`)))
  (set `CharacterMovementComponent.MaxFlySpeed` _returnvalue _charactermovement)
  (set `CharacterMovementComponent.MaxWalkSpeed` _returnvalue _charactermovement))

(fn `UserConstructionScript`
  (`CharacterMovementComponent.SetMovementMode` (`self.CharacterMovement`) "MOVE_Walking" 0))